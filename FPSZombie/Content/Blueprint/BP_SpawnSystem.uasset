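; Spawner Blueprint that spawns a wave of BP_Zombie actors across four box areas.
; SpawnZombies runs a delayed loop with short randomized pauses, its inclusive zero-based range yielding one more iteration than NumEnemies.
; Each iteration passes a random index to GetRandomSpawnerLocation, which selects one of four Box functions built around random points in the spawn boxes.
; Spawning ignores collisions, and a CustomForDelay macro implements a Delay-based for loop.
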(event Custom|SpawnZombies
  (params (NumEnemies :type Integer))
  (Utilities|ForLoopwithDelay 0 NumEnemies (Math|Random|RandomFloatinRange 0.2 0.5)
    (:Loop%20body
      (bind _output (CallFunction|GetRandomSpawnerLocation (Math|Random|RandomIntegerinRange 0 3)))
      (Game|SpawnActorfromClass "/Game/Blueprints_Iván/BP_Zombie.BP_Zombie_C" _output "AlwaysSpawn" 0 0))))

(fn ConstructionScript)

(fn GetRandomSpawnerLocation
  (params (Spawner :type Integer))
  (switch int Spawner
    (:0
      (LocalVariables|SetLocationOutput (|Box01)))
    (:1
      (LocalVariables|SetLocationOutput (|Box02)))
    (:2
      (LocalVariables|SetLocationOutput (|Box03)))
    (:3
      (LocalVariables|SetLocationOutput (|Box04))))
  (return (LocalVariables|GetLocationOutput)))