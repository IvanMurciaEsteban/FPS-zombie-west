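; BP_WaveControl is a wave controller that starts a zombie wave when play begins.
; StartWave checks ActualWave against NumWaves, passes the enemy count at index ActualWave + 1 of NumEnemiesWave to the Spawner's SpawnZombies, then increments ActualWave.
; This Blueprint calls StartWave only from BeginPlay and has no logic of its own to trigger later waves.
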(event EventBeginPlay
  (CallFunction|StartWave))

(event Collision|EventActorBeginOverlap
  (params (OtherActor :type Actor%20Object%20Reference)))

(event EventTick
  (params (DeltaSeconds :type Float%20%28single-precision%29)))

(fn ConstructionScript)

(fn StartWave
  (if (< (Variables|Default|GetActualWave) (Variables|Default|GetNumWaves))
    (Default|SpawnZombies (Variables|Default|GetSpawner) (Utilities|Array|Get(acopy) (Variables|Default|GetNumEnemies_Wave) (+ (Variables|Default|GetActualWave) 1)))
    (Variables|Default|SetActualWave (+ (Variables|Default|GetActualWave) 1))))