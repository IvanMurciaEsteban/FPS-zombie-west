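; Zombie enemy that attacks the saloon and can be shot dead by first-person projectiles.
; MoveToSaloon re-issues an AI move every three seconds until the zombie attacks, but its startup call and saloon lookup are disconnected.
; Overlapping the saloon stops movement and starts a delayed loop that drains its Life and calls CheckLife.
; Head hits kill instantly, while body hits decrement the zombie's Life until it is destroyed.
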(event OnComponentHit(BodyHitBox)
  (params (HitComponent :type Primitive%20Component%20Object%20Reference) (OtherActor :type Actor%20Object%20Reference) (OtherComp :type Primitive%20Component%20Object%20Reference) (NormalImpulse :type Vector :default "0, 0, 0") (Hit :type Hit%20Result%20Structure%20%28by%20ref%29))
  ;[1 1 1] DamageReceive
  ;;[1 1 1] Cambiar por la "bala" definitiva
  (Utilities|Casting|CastToBP_FirstPersonProjectile OtherActor)
  (bind _result (Math|Integer|DecrementInt (Variables|Default|GetLife))
    (:%20%20
      (Actor|DestroyActor OtherActor)
      (if (<= _result 0)
        (Actor|DestroyActor)))))

(event OnComponentHit(HeadHitBox)
  (params (HitComponent :type Primitive%20Component%20Object%20Reference) (OtherActor :type Actor%20Object%20Reference) (OtherComp :type Primitive%20Component%20Object%20Reference) (NormalImpulse :type Vector :default "0, 0, 0") (Hit :type Hit%20Result%20Structure%20%28by%20ref%29))
  ;[1 1 1] DamageReceive
  ;;[1 1 1] Cambiar por la "bala" definitiva
  (Utilities|Casting|CastToBP_FirstPersonProjectile OtherActor)
  (Actor|DestroyActor OtherActor)
  (Actor|DestroyActor))

(event Custom|Event%20StartAttack
  ;[1 1 1] Saloon Damage
  (bind _asbp_saloon (Utilities|Casting|CastToBP_Saloon (stale Collision|EventActorBeginOverlap OtherActor)))
  (bind _result (Math|Integer|DecrementInt (Variables|/Game/BlueprintsDani/BP_Saloon.BP_Saloon_C|GetLife _asbp_saloon))
    (:%20%20
      (Default|EventCheckLife _asbp_saloon)
      (Development|PrintString (Utilities|String|ToString(Integer) _result) true true "(R=0.053151,G=1.000000,B=0.000000,A=1.000000)")
      (Utilities|FlowControl|Delay 1.0)
      (CallFunction|EventStartAttack))))

(event Custom|Event%20MoveToSaloon
  (if (not (Variables|Default|GetisAttacking))
    (AI|AIMoveTo self (Variables|Default|GetSaloonLocation) 0 1e+02 false
      (:then
        (Utilities|FlowControl|Delay 3.0)
        (CallFunction|EventMovetoSaloon self)))))

(event EventTick
  (params (DeltaSeconds :type Float%20%28single-precision%29)))

(event Collision|EventActorBeginOverlap
  (params (OtherActor :type Actor%20Object%20Reference))
  ;[1 1 1] Saloon Damage
  (Utilities|Casting|CastToBP_Saloon OtherActor)
  (Development|PrintString "Saloon")
  (Components|Movement|StopMovementImmediately (Variables|Character|GetCharacterMovement))
  (Variables|Default|SetisAttacking true)
  (CallFunction|EventStartAttack))

(event EventBeginPlay)

(fn ConstructionScript)