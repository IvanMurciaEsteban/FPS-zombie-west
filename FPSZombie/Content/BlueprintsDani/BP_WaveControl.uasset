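; Wave controller for a zombie game with tower placement, driving numbered waves and the interludes between them.
; StartWave clears the player's previous tower, ends the interlude and, while waves remain, has Spawner create that wave's enemy count with exponentially growing health.
; CheckZombiesLeft counts down to wave completion, which opens an interlude and starts the next wave after a delay that lengthens in later waves.
; BeginPlay is empty, so nothing here triggers the first wave.
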(event Custom|Event%20WaitNextWave
  (if (<= (Variables|Default|GetActualWave) 5)
    (Utilities|FlowControl|Delay 6e+01)
    (else
      (Utilities|FlowControl|Delay 1.2e+02)))
  (CallFunction|StartWave))

(event EventBeginPlay)

(event Collision|EventActorBeginOverlap
  (params (OtherActor :type Actor%20Object%20Reference)))

(event EventTick
  (params (DeltaSeconds :type Float%20%28single-precision%29)))

(fn ConstructionScript)

(fn StartWave
  (bind _outactors (Actor|GetAllActorsOfClass "/Game/FirstPerson_Dani/BlueprintsDani/BP_FirstPersonCharacter_Dani.BP_FirstPersonCharacter_Dani_C"))
  (Default|RemovePreviousTower (Utilities|Array|Get(acopy) _outactors) (Variables|/Game/FirstPerson_Dani/BlueprintsDani/BP_FirstPersonCharacter_Dani.BP_FirstPersonCharacter_Dani_C|GetSpawnActor (Utilities|Array|Get(acopy) _outactors)))
  (Variables|Default|SetInterlude false)
  (if (< (Variables|Default|GetActualWave) (Variables|Default|GetNumWaves))
    (bind _output_get (Variables|Default|SetZombiesLeft (Utilities|Array|Get(acopy) (Variables|Default|GetNumEnemies_Wave) (Variables|Default|GetActualWave))))
    (bind _output_get_2 (Variables|Default|SetZombieLife (* (Math|Float|Power 1.05 (Math|Conversions|ToFloat(Integer) (Variables|Default|GetActualWave))) 1e+02)))
    (Default|SpawnZombies (Variables|Default|GetSpawner) (Utilities|Array|Get(acopy) (Variables|Default|GetNumEnemies_Wave) (Variables|Default|GetActualWave)) _output_get_2)
    (Variables|Default|SetActualWave (+ (Variables|Default|GetActualWave) 1))
    (Development|PrintString (Utilities|String|Append "Oleada: " (Utilities|String|ToString(Integer) (Variables|Default|GetActualWave))))
    (Development|PrintString (Utilities|String|Append "Total Zombies: " (Utilities|String|ToString(Integer) _output_get)))))

(fn CheckZombiesLeft
  (bind _result (Math|Integer|DecrementInt (Variables|Default|GetZombiesLeft))
    (:%20%20
      (bind _output_get (Variables|Default|SetZombiesLeft _result))
      (Development|PrintString (Utilities|String|Append "Quedan: " (Utilities|String|ToString(Integer) _output_get)))
      (if (<= _output_get 0)
        (CallFunction|WaveCompleted)))))

(fn WaveCompleted
  (Development|PrintString "Oleada Completada")
  (Variables|Default|SetInterlude true)
  (CallFunction|EventWaitNextWave))