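; Zombie enemy that walks to the saloon and attacks it, draining its life.
; On BeginPlay it finds BP_Saloon and uses AI MoveTo toward its sphere; overlapping the saloon stops movement and starts a one-second damage loop with debug prints.
; A Damage function applies normal or critical hits, and CheckAlive destroys the zombie at zero life and notifies BP_WaveControl.
; Head and body hitbox hit events are empty, leaving old bullet logic disconnected.
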(event OnComponentHit(BodyHitBox)
  (params (HitComponent :type Primitive%20Component%20Object%20Reference) (OtherActor :type Actor%20Object%20Reference) (OtherComp :type Primitive%20Component%20Object%20Reference) (NormalImpulse :type Vector :default "0, 0, 0") (Hit :type Hit%20Result%20Structure%20%28by%20ref%29))
  ;[1 1 1] DamageReceive
)

(event OnComponentHit(HeadHitBox)
  (params (HitComponent :type Primitive%20Component%20Object%20Reference) (OtherActor :type Actor%20Object%20Reference) (OtherComp :type Primitive%20Component%20Object%20Reference) (NormalImpulse :type Vector :default "0, 0, 0") (Hit :type Hit%20Result%20Structure%20%28by%20ref%29))
  ;[1 1 1] DamageReceive
)

(event Custom|Event%20StartAttack
  ;[1 1 1] Saloon Damage
  (bind _asbp_saloon (Utilities|Casting|CastToBP_Saloon (stale Collision|EventActorBeginOverlap OtherActor)))
  (bind _result (Math|Integer|DecrementInt (Variables|/Game/BlueprintsDani/BP_Saloon.BP_Saloon_C|GetLife _asbp_saloon))
    (:%20%20
      (Default|EventCheckLife _asbp_saloon)
      (Development|PrintString (Utilities|String|ToString(Integer) _result) true true "(R=0.053151,G=1.000000,B=0.000000,A=1.000000)")
      (Utilities|FlowControl|Delay 1.0)
      (CallFunction|EventStartAttack))))

(event Custom|Event%20MoveToSaloon
  (bind _saloonlocation (Variables|Default|GetSaloonLocation))
  (if (not (Variables|Default|GetisAttacking))
    (AI|AIMoveTo self (Math|Vector|MakeVector (.x _saloonlocation) (.y _saloonlocation) 0.0) 0 1e+02 false
      (:then
        (Utilities|FlowControl|Delay 3.0)
        (CallFunction|EventMovetoSaloon self)))))

(event Custom|Spawn)

(event EventBeginPlay
  (bind _outactors (Actor|GetAllActorsOfClass "/Game/BlueprintsDani/BP_Saloon.BP_Saloon_C"))
  (Variables|Default|SetSaloonLocation (Transformation|GetWorldLocation (Variables|/Game/BlueprintsDani/BP_Saloon.BP_Saloon_C|GetSphere (Utilities|Array|Get(acopy) _outactors))))
  (CallFunction|EventMovetoSaloon))

(event EventTick
  (params (DeltaSeconds :type Float%20%28single-precision%29)))

(event Collision|EventActorBeginOverlap
  (params (OtherActor :type Actor%20Object%20Reference))
  ;[1 1 1] Saloon Damage
  (bind _asbp_saloon (Utilities|Casting|CastToBP_Saloon OtherActor))
  (Development|PrintString (Utilities|GetDisplayName _asbp_saloon))
  (Components|Movement|StopMovementImmediately (Variables|Character|GetCharacterMovement))
  (Variables|Default|SetisAttacking true)
  (CallFunction|EventStartAttack))

(fn ConstructionScript)

(fn Damage
  (params (Damage :type Float%20%28double-precision%29) (Crit :type Boolean))
  (if Crit
    (bind _output_get (Variables|Default|SetLife (- (Variables|Default|GetLife) (* (LocalVariables|GetCRITIC_MULTIPLY) Damage))))
    (CallFunction|CheckAlive _output_get)
    (else
      (bind _output_get_2 (Variables|Default|SetLife (- (Variables|Default|GetLife) Damage)))
      (CallFunction|CheckAlive _output_get_2))))

(fn CheckAlive
  (params (Health :type Float%20%28double-precision%29))
  (if (<= Health 0.0)
    (Actor|DestroyActor)
    (bind _outactors (Actor|GetAllActorsOfClass "/Game/BlueprintsDani/BP_WaveControl.BP_WaveControl_C"))
    (Default|CheckZombiesLeft (Utilities|Array|Get(acopy) _outactors))))