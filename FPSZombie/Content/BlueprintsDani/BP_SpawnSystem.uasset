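; Zombie spawner whose SpawnZombies event spawns a given number of BP_Zombie_Ivan_Dani actors, setting each one's Life.
; A delayed loop staggers spawns by random intervals, with GetRandomSpawnerLocation selecting one of four Box functions at random for the transform.
; Each Box function holds a random-point-in-bounds calculation for its spawn area, shown unconnected to any output.
; A CustomForDelay macro defines a delayed counting loop.
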(event Custom|SpawnZombies
  (params (NumEnemies :type Integer) (ZombieLife :type Float%20%28double-precision%29))
  (Utilities|ForLoopwithDelay 1 NumEnemies (Math|Random|RandomFloatinRange 0.5 1.5)
    (:Loop%20body
      (bind _output (CallFunction|GetRandomSpawnerLocation (Math|Random|RandomIntegerinRange 0 3)))
      (bind _returnvalue (Game|SpawnActorfromClass "/Game/BlueprintsDani/BP_Zombie_Ivan_Dani.BP_Zombie_Ivan_Dani_C" _output "AdjustIfPossibleButAlwaysSpawn" 0 0))
      (Variables|/Game/BlueprintsDani/BP_Zombie_Ivan_Dani.BP_Zombie_Ivan_Dani_C|SetLife _returnvalue ZombieLife))))

(fn ConstructionScript)

(fn GetRandomSpawnerLocation
  (params (Spawner :type Integer))
  (switch int Spawner
    (:0
      (LocalVariables|SetLocationOutput (|Box01)))
    (:1
      (LocalVariables|SetLocationOutput (|Box02)))
    (:2
      (LocalVariables|SetLocationOutput (|Box03)))
    (:3
      (LocalVariables|SetLocationOutput (|Box04))))
  (return (LocalVariables|GetLocationOutput)))