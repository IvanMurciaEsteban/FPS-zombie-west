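; BP_Tower is a placeable tower actor that previews whether its current position is valid before it is placed.
; CheckSpawn sets CanSpawn false and shows a red material if any actor overlaps it, otherwise true with a green one.
; Place, when CanSpawn is true, applies the Material variable to the mesh and switches its collision to BlockAllDynamic.
; Its own event graph is empty, so both functions rely on external callers.
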(event EventBeginPlay)

(event Collision|EventActorBeginOverlap
  (params (OtherActor :type Actor%20Object%20Reference)))

(event EventTick
  (params (DeltaSeconds :type Float%20%28single-precision%29)))

(fn ConstructionScript)

(fn CheckSpawn
  (bind _mesh (Variables|Default|GetMesh))
  (if (> (Utilities|Array|Length (Collision|GetOverlappingActors 0 :!class /Script/Engine.Actor)) 0)
    (Rendering|Material|SetMaterial _mesh 0 "/Game/BlueprintsDani/Towers/PlaceTower/M_RedPlace.M_RedPlace")
    (Variables|Default|SetCanSpawn false)
    (else
      (Rendering|Material|SetMaterial _mesh 0 "/Game/BlueprintsDani/Towers/PlaceTower/M_GreenPlace.M_GreenPlace")
      (Variables|Default|SetCanSpawn true))))

(fn Place
  (bind _mesh (Variables|Default|GetMesh))
  (if (Variables|Default|GetCanSpawn)
    (Rendering|Material|SetMaterial _mesh 0 (Variables|Default|GetMaterial))
    (Collision|SetCollisionProfileName _mesh "BlockAllDynamic" true :!class /Script/Engine.PrimitiveComponent)))