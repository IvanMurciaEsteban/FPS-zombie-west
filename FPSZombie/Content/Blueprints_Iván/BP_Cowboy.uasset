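; BP_Cowboy is a cowboy shooter that attacks zombies with a pistol.
; AttackZombie plays the shoot montage on the mesh, then calls SoundAndAnimation and applies fixed, non-critical damage to the passed Zombie.
; SoundAndAnimation plays the Colt shot at the given location and attaches a muzzle flash to the Emmiter component, with its pitch flipped 180 degrees.
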(event Custom|AttackZombie
  (params (Zombie :type BP%20Zombie%20Object%20Reference))
  (Animation|Montage|PlayMontage (Variables|Character|GetMesh) "/Game/Blueprints_Iván/Helper/Shoot_Montage.Shoot_Montage" 1.5
    (:then
      (|SoundAndAnimation (Transformation|GetWorldLocation (Variables|Character|GetMesh))
        (:Out
          (Default|Damage Zombie 5e+01 false))))))

(fn ConstructionScript)