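; BP_TowerSupport is a purchasable support building that spawns BP_Cowboy actors at its spawn points.
; Its PlayerCollider overlap registers the building as the first-person character's HouseBuy and toggles CanBuy and the buy text on entry and exit.
; SpawnCowboy, not called within this Blueprint, decrements AvailableSpots and uses the remaining count to place a cowboy at Spawn01, then Spawn02.
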(event OnComponentBeginOverlap(PlayerCollider)
  (params (OverlappedComponent :type Primitive%20Component%20Object%20Reference) (OtherActor :type Actor%20Object%20Reference) (OtherComp :type Primitive%20Component%20Object%20Reference) (OtherBodyIndex :type Integer) (bFromSweep :type Boolean) (SweepResult :type Hit%20Result%20Structure%20%28by%20ref%29))
  (bind _asbp_first_person_character (Utilities|Casting|CastToBP_FirstPersonCharacter OtherActor))
  (Variables|/Game/FirstPerson/Blueprints_Iván/BP_FirstPersonCharacter.BP_FirstPersonCharacter_C|SetHouseBuy _asbp_first_person_character self)
  (Variables|/Game/FirstPerson/Blueprints_Iván/BP_FirstPersonCharacter.BP_FirstPersonCharacter_C|SetCanBuy _asbp_first_person_character true)
  (Default|ShowBuyText _asbp_first_person_character))

(event OnComponentEndOverlap(PlayerCollider)
  (params (OverlappedComponent :type Primitive%20Component%20Object%20Reference) (OtherActor :type Actor%20Object%20Reference) (OtherComp :type Primitive%20Component%20Object%20Reference) (OtherBodyIndex :type Integer))
  (bind _asbp_first_person_character (Utilities|Casting|CastToBP_FirstPersonCharacter OtherActor))
  (Variables|/Game/FirstPerson/Blueprints_Iván/BP_FirstPersonCharacter.BP_FirstPersonCharacter_C|SetCanBuy _asbp_first_person_character false)
  (Default|HideBuyText _asbp_first_person_character))

(event EventBeginPlay)

(event Collision|EventActorBeginOverlap
  (params (OtherActor :type Actor%20Object%20Reference)))

(event EventTick
  (params (DeltaSeconds :type Float%20%28single-precision%29)))

(fn ConstructionScript)

(fn SpawnCowboy
  (bind _output_get (Variables|Default|SetAvailableSpots (- (Variables|Default|GetAvailableSpots) 1)))
  (switch int _output_get
    (:0
      (Game|SpawnActorfromClass "/Game/Blueprints_Iván/BP_Cowboy.BP_Cowboy_C" (Transformation|GetWorldTransform (Variables|Default|GetSpawn02)) "Undefined" 0 0))
    (:1
      (Game|SpawnActorfromClass "/Game/Blueprints_Iván/BP_Cowboy.BP_Cowboy_C" (Transformation|GetWorldTransform (Variables|Default|GetSpawn01)) "Undefined" 0 0))))