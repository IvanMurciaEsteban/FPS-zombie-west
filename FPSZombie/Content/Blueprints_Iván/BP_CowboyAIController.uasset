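; AI controller for the cowboy that runs BT_Cowboy and feeds it zombie targets through AI Perception.
; Without a target, a perception update on a BP_Zombie writes it to the Target blackboard key and sets hasTarget from the sensing result.
; With a target, updates only clear hasTarget when the updated zombie is dead, without checking that it is the stored Target.
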(event OnTargetPerceptionUpdated(AIPerception)
  (params (Actor :type Actor%20Object%20Reference) (Stimulus :type AI%20Stimulus%20Structure))
  (bind _returnvalue (Utilities|Name|MakeLiteralName "hasTarget"))
  (bind _blackboard (Variables|Default|GetBlackboard))
  (bind _asbp_zombie (Utilities|Casting|CastToBP_Zombie Actor))
  (if (ScalableFloat|GetValueasBool (Variables|Default|GetBlackboard) (Utilities|Name|MakeLiteralName "hasTarget"))
    (if (Variables|/Game/Blueprints_Iván/BP_Zombie.BP_Zombie_C|GetisDeath _asbp_zombie)
      (AI|Components|Blackboard|SetValueasBool _blackboard _returnvalue false))
    (else
      (AI|Components|Blackboard|SetValueasBool _blackboard _returnvalue (.bSuccessfullySensed (Utilities|Struct|BreakAIStimulus Stimulus)))
      (AI|Components|Blackboard|SetValueasObject _blackboard (Utilities|Name|MakeLiteralName "Target") _asbp_zombie))))

(event EventBeginPlay
  (AI|RunBehaviorTree "/Game/Blueprints_Iván/BT_Cowboy.BT_Cowboy"))

(fn ConstructionScript)